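; Double-sided road segment Actor that supports continuous road spawning as the player moves along X.
; A Character overlapping its Box trigger calls SpawnRoad on the referenced road spawner.
; Each Tick it destroys itself once its X is below the player's and their absolute X values differ by more than a fixed margin.
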(event `self.ReceiveTick`
  (params (DeltaSeconds :type "Float (single-precision)"))
  (bind _returnvalue_x (`KismetMathLibrary.BreakVector` (`self.K2_GetActorLocation`)))
  (bind _returnvalue_x_2 (`KismetMathLibrary.BreakVector` (`self.K2_GetActorLocation`)))
  (bind _returnvalue_x_3 (`KismetMathLibrary.BreakVector` (`self.K2_GetActorLocation` (`GameplayStatics.GetPlayerCharacter` 0))))
  (bind _returnvalue_x_4 (`KismetMathLibrary.BreakVector` (`self.K2_GetActorLocation` (`GameplayStatics.GetPlayerCharacter` 0))))
  (if (and (< _returnvalue_x_2 _returnvalue_x_4) (> (- (`KismetMathLibrary.Abs` _returnvalue_x_3) (`KismetMathLibrary.Abs` _returnvalue_x)) 500.0))
    (`self.K2_DestroyActor`)))

(event `self.ReceiveActorBeginOverlap`
  (params (OtherActor :type "Actor Object Reference")))

(event `self.Box.OnComponentBeginOverlap`
  (params (OverlappedComponent :type "PrimitiveComponent Object Reference") (OtherActor :type "Actor Object Reference") (OtherComp :type "PrimitiveComponent Object Reference") (OtherBodyIndex :type Integer) (bFromSweep :type Boolean) (SweepResult :type "HitResult Structure (by ref)"))
  (cast `Character` OtherActor)
  (`/Game/Blueprints/road_spawner.spawn_road` (`self.road_spawner_ref`)))

(fn `UserConstructionScript`)