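; Left spawner actor that periodically spawns police car actors at its own position.
; Tick serves as the timer, with its interval re-randomized between two short delays on BeginPlay and on every tick.
; Each tick passes two coin flips, a one-in-four chance, before spawning a PoliceCarActor at the spawner's X/Y with fixed height and zero rotation.
; BeginPlay also picks a random Mult value, which nothing in this graph reads.
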(event `self.ReceiveBeginPlay`
  (`self.SetActorTickInterval` (select `int` (`KismetMathLibrary.RandomIntegerInRange` 0 1) :`0` 2.0 :`1` 3.0 :!type "Float (single-precision)"))
  (set `self.mult` (select `int` (`KismetMathLibrary.RandomIntegerInRange` 0 3) :`0` 2 :`1` 3 :`2` 4 :`3` 5)))

(event `self.ReceiveTick`
  (params (DeltaSeconds :type "Float (single-precision)"))
  (bind (_returnvalue_x _returnvalue_y) (`KismetMathLibrary.BreakVector` (`self.K2_GetActorLocation`)))
  (`self.SetActorTickInterval` (select `int` (`KismetMathLibrary.RandomIntegerInRange` 0 1) :`0` 2.0 :`1` 3.0 :!type "Float (single-precision)"))
  (`|ExecutionSequence`
    (:`then_0`
      (if (== (`KismetMathLibrary.RandomIntegerInRange` 0 1) 0)
        (if (== (`KismetMathLibrary.RandomIntegerInRange` 0 1) 0)
          (`|SpawnActorFromClass` "/Game/Blueprints/PoliceCarActor.PoliceCarActor_C" (`KismetMathLibrary.MakeTransform` (`KismetMathLibrary.MakeVector` _returnvalue_x _returnvalue_y -20.0) (struct)) "Undefined" "OverrideRootScale" null null))))))

(fn `UserConstructionScript`)