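; Road spawner that extends the level along X with DoubleSidedRoadActor pieces and vehicle spawners.
; SpawnRoad places a road piece, makes two SpawnVehicle attempts at offsets behind it, then advances SpawnLocX and places another piece holding a reference back to this spawner.
; Each attempt has a 50% chance of creating a Left_spawner.
; SpawnBarriers is an empty stub, and nothing in this Blueprint calls SpawnRoad.
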(fn `spawn_barriers`)

(fn `spawn_left`
  (`|SpawnActorFromClass` "/Game/Blueprints/left_spawner.left_spawner_C" (`KismetMathLibrary.MakeTransform` (`KismetMathLibrary.MakeVector` (`self.vehicle_spawn_loc_x`) -700.0)) "Undefined" "OverrideRootScale" null null))

(fn `spawn_road`
  (`|SpawnActorFromClass` "/Game/Blueprints/DoubleSidedRoadActor.DoubleSidedRoadActor_C" (`KismetMathLibrary.MakeTransform` (`KismetMathLibrary.MakeVector` (`self.spawn_loc_x`) -590.0 (`self.road_z`))) "Undefined" "OverrideRootScale" null null)
  (`|ExecutionSequence`
    (:`then_0`
      (set `self.vehicle_spawn_loc_x` (- (`self.spawn_loc_x`) 75.0))
      (`self.spawn_vehicle`))
    (:`then_1`
      (set `self.vehicle_spawn_loc_x` (- (`self.vehicle_spawn_loc_x`) 70.0))
      (`self.spawn_vehicle`)
      (bind _output_get (set `self.spawn_loc_x` (+ (`self.spawn_loc_x`) 160.0)))
      (bind _returnvalue (`|SpawnActorFromClass` "/Game/Blueprints/DoubleSidedRoadActor.DoubleSidedRoadActor_C" (`KismetMathLibrary.MakeTransform` (`KismetMathLibrary.MakeVector` _output_get 0.0 (`self.road_z`))) "Undefined" "OverrideRootScale" null null))
      (set `/Game/Blueprints/DoubleSidedRoadActor.road_spawner_ref` self _returnvalue))))

(fn `spawn_vehicle`
  (if (== (`KismetMathLibrary.RandomIntegerInRange` 0 1) 0)
    (`self.spawn_left`)))

(fn `UserConstructionScript`)